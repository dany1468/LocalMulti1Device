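; BP_PlayerCharacter is a player character Blueprint with a name label and a physics push on a sphere component.
; SetPlayerName copies the actor's first tag into the TextRender as the displayed name.
; Push applies a mass-independent force to the Sphere along the sphere's own forward vector.
; Both are custom events, and nothing in this Blueprint calls them.
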(event `SetPlayerName`
  (`TextRenderComponent.K2_SetText` (`self.TextRender`) (`KismetTextLibrary.Conv_NameToText` (`|GetArrayItem` (`self.Tags`)))))

(event `Push`
  (`PrimitiveComponent.AddForce` (`self.Sphere`) (* (`SceneComponent.GetForwardVector` (`self.Sphere`)) 3000.0) "None" true))

(fn `UserConstructionScript`)