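; PC_SingleView is a player controller that lets a single local input setup drive two player characters.
; On BeginPlay it adds the default Enhanced Input mapping context, then finds the characters tagged Player1 and Player2, stores them and sets their names.
; Separate 1P and 2P push input actions call Push on the matching character.
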(event `self.ReceiveBeginPlay`
  (bind _returnvalue (subsystem `EnhancedInputLocalPlayerSubsystem`))
  (`|ExecutionSequence`
    (:`then_0`
      (`/Engine/EditorBlueprintResources/StandardMacros.IsValid` _returnvalue
        (:`Is Valid`
          (`EnhancedInputSubsystemInterface.AddMappingContext` _returnvalue "/Game/Inputs/IMC_Default.IMC_Default" 0 (make `ModifyContextOptions` true)))))
    (:`then_1`
      (bind _outactors (`GameplayStatics.GetAllActorsWithTag` "Player1"))
      (bind _asbp_player_character (cast `/Game/BP_PlayerCharacter` (`|GetArrayItem` _outactors)))
      (bind _output_get (set `self.Player1` _asbp_player_character))
      (`/Game/BP_PlayerCharacter.SetPlayerName` _output_get))
    (:`then_2`
      (bind _outactors_2 (`GameplayStatics.GetAllActorsWithTag` "Player2"))
      (bind _asbp_player_character_2 (cast `/Game/BP_PlayerCharacter` (`|GetArrayItem` _outactors_2)))
      (bind _output_get_2 (set `self.Player2` _asbp_player_character_2))
      (`/Game/BP_PlayerCharacter.SetPlayerName` _output_get_2))))

(event `EnhancedInput|/Game/Inputs/IA_Push1P`
  (params (ActionValue :type Boolean) (ElapsedSeconds :type "Float (double-precision)") (TriggeredSeconds :type "Float (double-precision)") (InputAction :type "InputAction Object Reference" :default "/Game/Inputs/IA_Push1P.IA_Push1P"))
  (:`Triggered`
    (`/Game/BP_PlayerCharacter.Push` (`self.Player1`))))

(event `EnhancedInput|/Game/Inputs/IA_Push2P`
  (params (ActionValue :type Boolean) (ElapsedSeconds :type "Float (double-precision)") (TriggeredSeconds :type "Float (double-precision)") (InputAction :type "InputAction Object Reference" :default "/Game/Inputs/IA_Push2P.IA_Push2P"))
  (:`Triggered`
    (`/Game/BP_PlayerCharacter.Push` (`self.Player2`))))

(fn `UserConstructionScript`)