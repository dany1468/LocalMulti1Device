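; Game mode for a two-player separate-view setup, driven by two PC_SeparateViewWithPlayerStart controllers.
; On BeginPlay it creates a second local player, caches both controllers, and waits briefly before initializing.
; InitPlayer has each controller set an index and tag and return its character, then registers both characters with the first controller, which then initializes as the main controller.
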(event `self.ReceiveBeginPlay`
  ;[1 1 1] Player2
  (bind _returnvalue (`GameplayStatics.CreatePlayer` -1))
  (bind _aspc_separate_view_with_player_start (cast `/Game/SeparateView/PC_SeparateViewWithPlayerStart` _returnvalue))
  (set `self.PlayerController2` _aspc_separate_view_with_player_start)
  ;[1 1 1] Player1
  (bind _aspc_separate_view_with_player_start_2 (cast `/Game/SeparateView/PC_SeparateViewWithPlayerStart` (`GameplayStatics.GetPlayerController` 0)))
  (set `self.PlayerController1` _aspc_separate_view_with_player_start_2)
  (`KismetSystemLibrary.Delay` 0.5)
  (`self.Init Player`)
  (`/Game/SeparateView/PC_SeparateViewWithPlayerStart.InitMainController` (`self.PlayerController1`)))

(event `Init Player`
  ;[1 1 1 1 14] 各 Controller が保有するキャラクターのパラメータを設定し参照を取得
  (bind _playercharacter (`/Game/SeparateView/PC_SeparateViewWithPlayerStart.SetPlayerParams` (`self.PlayerController1`) 0 "Player1"))
  (bind _playercharacter_2 (`/Game/SeparateView/PC_SeparateViewWithPlayerStart.SetPlayerParams` (`self.PlayerController2`) 1 "Player2"))
  ;[1 1 1 1 14] PlayerController1 にそれぞれのキャラクターを登録
  (`/Game/SeparateView/PC_SeparateViewWithPlayerStart.RegisterPlayers` (`self.PlayerController1`) _playercharacter _playercharacter_2))

(fn `UserConstructionScript`)